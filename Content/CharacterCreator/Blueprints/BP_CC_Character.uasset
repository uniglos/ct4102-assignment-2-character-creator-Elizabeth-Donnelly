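; Modular character for a character creator, built from head, body, legs and feet skeletal meshes, with events to swap each part.
; The construction script chains leader poses, with body following head and legs and feet following body.
; It also resets head material slots and stores dynamic instances of those matching the hair material in HairMaterials.
; On BeginPlay it adds the character UI to the viewport.
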(event Custom|SwapHead
  (params (Head :type Skeletal%20Mesh%20Object%20Reference))
  (Components|SkeletalMesh|SetSkeletalMeshAsset (Variables|Default|GetHead) Head))

(event Custom|SwapBody
  (params (Body :type Skeletal%20Mesh%20Object%20Reference))
  (Components|SkeletalMesh|SetSkeletalMeshAsset (Variables|Default|GetBody) Body))

(event Custom|SwapLegs
  (params (Legs :type Skeletal%20Mesh%20Object%20Reference))
  (Components|SkeletalMesh|SetSkeletalMeshAsset (Variables|Default|GetLegs) Legs))

(event Custom|SwapFeet
  (params (Feet :type Skeletal%20Mesh%20Object%20Reference))
  (Components|SkeletalMesh|SetSkeletalMeshAsset (Variables|Default|GetFeet) Feet))

(event Collision|EventActorBeginOverlap
  (params (OtherActor :type Actor%20Object%20Reference)))

(event EventTick
  (params (DeltaSeconds :type Float%20%28single-precision%29)))

(event EventBeginPlay
  (bind _returnvalue (UserInterface|CreateWidget "/Game/CharacterCreator/UI/CharacterUI.CharacterUI_C"))
  (UserInterface|Viewport|AddtoViewport _returnvalue 0))

(fn ConstructionScript
  (bind _body (Variables|Default|GetBody))
  (bind _head (Variables|Default|GetHead))
  (bind _hairmaterials (Variables|Default|GetHairMaterials))
  (Components|SkinnedMesh|SetLeaderPoseComponent _body (Variables|Default|GetHead) false false)
  (Components|SkinnedMesh|SetLeaderPoseComponent (Variables|Default|GetLegs) _body false false)
  (Components|SkinnedMesh|SetLeaderPoseComponent (Variables|Default|GetFeet) _body false false)
  (Utilities|Array|Clear _hairmaterials)
  (for (_ _array_index) (Rendering|Material|GetMaterials _head)
    (Rendering|Material|SetMaterial _head _array_index 0)
    (if (== (Rendering|Material|GetMaterial _head _array_index) "/Game/ModularPack/Materials/Hair.Hair")
      (bind _returnvalue (Rendering|Material|CreateDynamicMaterialInstance _head _array_index "/Game/ModularPack/Materials/Hair.Hair" "HairColour" :!class /Script/Engine.PrimitiveComponent))
      (Utilities|Array|Add _hairmaterials _returnvalue))))